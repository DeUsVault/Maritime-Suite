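; Man-of-war ship pawn driven by physics forces, with manual keyboard control or Space-toggled autopilot, plus numpad-switched cameras with wheel zoom.
; Keys or AI set left, right and steering flags, which Tick ramps into forces applied at three points on MainBox.
; The autopilot follows Path spline points, turning with opposed side forces until aligned, then advancing.
; UpdateLonLat and Radar are empty stubs; damage and destruction only print debug text.
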(event `Key|NumPadFive`
  (params (Key :type "Key Structure"))
  ;[1 1 1] Toggle Cameras
  (:`Pressed`
    (`self.Toggle Cameras` 5)))

(event `Key|NumPadZero`
  (params (Key :type "Key Structure"))
  ;[1 1 1] Toggle Cameras
  (:`Pressed`
    (`self.Toggle Cameras` 0)))

(event `Key|NumPadSix`
  (params (Key :type "Key Structure"))
  ;[1 1 1] Toggle Cameras
  (:`Pressed`
    (`self.Toggle Cameras` 6)))

(event `Key|NumPadOne`
  (params (Key :type "Key Structure"))
  ;[1 1 1] Toggle Cameras
  (:`Pressed`
    (`self.Toggle Cameras` 1)))

(event `Key|NumPadSeven`
  (params (Key :type "Key Structure"))
  ;[1 1 1] Toggle Cameras
  (:`Pressed`
    (`self.Toggle Cameras` 7)))

(event `Key|MouseScrollUp`
  (params (Key :type "Key Structure"))
  ;[1 1 1] Zoom In-Out
  (:`Pressed`
    (`self.ZoomInOut` false)))

(event `Key|NumPadTwo`
  (params (Key :type "Key Structure"))
  ;[1 1 1] Toggle Cameras
  (:`Pressed`
    (`self.Toggle Cameras` 2)))

(event `Key|MouseScrollDown`
  (params (Key :type "Key Structure"))
  ;[1 1 1] Zoom In-Out
  (:`Pressed`
    (`self.ZoomInOut` true)))

(event `Key|NumPadThree`
  (params (Key :type "Key Structure"))
  ;[1 1 1] Toggle Cameras
  (:`Pressed`
    (`self.Toggle Cameras` 3)))

(event `Key|NumPadEight`
  (params (Key :type "Key Structure"))
  ;[1 1 1] Toggle Cameras
  (:`Pressed`
    (`self.Toggle Cameras` 8)))

(event `Key|NumPadNine`
  (params (Key :type "Key Structure"))
  ;[1 1 1] Toggle Cameras
  (:`Pressed`
    (`self.Toggle Cameras` 9)))

(event `Key|NumPadFour`
  (params (Key :type "Key Structure"))
  ;[1 1 1] Toggle Cameras
  (:`Pressed`
    (`self.Toggle Cameras` 4)))

(event `Key|T`
  (params (Key :type "Key Structure"))
  (bind _forcesflag (`self.ForcesFlag`))
  ;[1 1 1] Left-Right Force Controls L:T-G-B, R:Y-H-N
  (:`Pressed`
    (`KismetArrayLibrary.Array_Set` _forcesflag 0 1))
  (:`Released`
    (`KismetArrayLibrary.Array_Set` _forcesflag)))

(event `Key|Y`
  (params (Key :type "Key Structure"))
  (bind _forcesflag (`self.ForcesFlag`))
  ;[1 1 1] Left-Right Force Controls L:T-G-B, R:Y-H-N
  (:`Pressed`
    (`KismetArrayLibrary.Array_Set` _forcesflag 1 1))
  (:`Released`
    (`KismetArrayLibrary.Array_Set` _forcesflag 1)))

(event `Key|I`
  (params (Key :type "Key Structure"))
  ;[1 1 1] Steering Controls: I-O-P
  (:`Pressed`
    (set `self.SteeringFlag` 1))
  (:`Released`
    (set `self.SteeringFlag` 0)))

(event `Key|O`
  (params (Key :type "Key Structure"))
  ;[1 1 1] Steering Controls: I-O-P
  (:`Pressed`
    (set `self.SteeringFlag` 3)))

(event `Key|G`
  (params (Key :type "Key Structure"))
  ;[1 1 1] Left-Right Force Controls L:T-G-B, R:Y-H-N
  (:`Pressed`
    (`KismetArrayLibrary.Array_Set` (`self.ForcesFlag`) 0 3)))

(event `Key|H`
  (params (Key :type "Key Structure"))
  ;[1 1 1] Left-Right Force Controls L:T-G-B, R:Y-H-N
  (:`Pressed`
    (`KismetArrayLibrary.Array_Set` (`self.ForcesFlag`) 1 3)))

(event `Key|P`
  (params (Key :type "Key Structure"))
  ;[1 1 1] Steering Controls: I-O-P
  (:`Pressed`
    (set `self.SteeringFlag` 2))
  (:`Released`
    (set `self.SteeringFlag` 0)))

(event `Key|B`
  (params (Key :type "Key Structure"))
  (bind _forcesflag (`self.ForcesFlag`))
  ;[1 1 1] Left-Right Force Controls L:T-G-B, R:Y-H-N
  (:`Pressed`
    (`KismetArrayLibrary.Array_Set` _forcesflag 0 2))
  (:`Released`
    (`KismetArrayLibrary.Array_Set` _forcesflag)))

(event `Key|N`
  (params (Key :type "Key Structure"))
  (bind _forcesflag (`self.ForcesFlag`))
  ;[1 1 1] Left-Right Force Controls L:T-G-B, R:Y-H-N
  (:`Pressed`
    (`KismetArrayLibrary.Array_Set` _forcesflag 1 2))
  (:`Released`
    (`KismetArrayLibrary.Array_Set` _forcesflag 1)))

(event `Key|SpaceBar`
  (params (Key :type "Key Structure"))
  (:`Released`
    (if (`self.AIPlay`)
      (set `self.AIPlay` false)
      (set `self.Status` "Manual")
      (else
        (set `self.AIPlay` true)
        (set `self.Status` "Auto")))))

(event `self.ReceiveTick`
  (params (DeltaSeconds :type "Float (single-precision)"))
  (`|ExecutionSequence`
    (:`then_0`
      (`self.updateLonLat`)
      (`self.Radar`))
    (:`then_1`
      (if (`self.AIPlay`)
        (`self.AI_Control`))
      (`self.SetForces`))
    (:`then_2`
      (`self.Apply Forces`))))

(event `self.ReceivePossessed`
  (params (NewController :type "Controller Object Reference"))
  (`self.Toggle Cameras` 0))

(event `self.ReceiveDestroyed`
  (`KismetSystemLibrary.PrintString` (`KismetStringLibrary.Conv_VectorToString` (`self.K2_GetActorLocation`)) true true (struct :`R` 0.083646 :`G` 1.0 :`A` 1.0) 20.0)
  (`KismetSystemLibrary.PrintString` "DESTROYED" true true (struct :`R` 1.0 :`G` 0.158633 :`A` 1.0) 20.0))

(event `self.ReceiveUnpossessed`
  (params (OldController :type "Controller Object Reference")))

(event `self.ReceiveAnyDamage`
  (params (Damage :type "Float (single-precision)") (DamageType :type "DamageType Object Reference") (InstigatedBy :type "Controller Object Reference") (DamageCauser :type "Actor Object Reference"))
  (`KismetSystemLibrary.PrintString` (`KismetStringLibrary.Concat_StrStr` "DAMAGED BY " (`KismetSystemLibrary.GetDisplayName` DamageCauser)) true true (struct :`G` 1.0 :`B` 0.036311 :`A` 1.0) 20.0))

(fn `AI Increase Force`
  (params (CurForce :type "Float (double-precision)") (Percentage :type "Float (double-precision)") (MaxMinForce :type "Float (double-precision)") (IsForward :type Boolean))
  (returns (Flag :type Integer))
  (locals (tmp_flag :type Integer))
  (if IsForward
    (if (>= CurForce (/ MaxMinForce Percentage))
      (set `local.tmp_flag` 0)
      (else
        (set `local.tmp_flag` 1)))
    (elif (<= CurForce (/ MaxMinForce Percentage))
      (set `local.tmp_flag` 0)
      (else
        (set `local.tmp_flag` 2))))
  (return (`local.tmp_flag`)))

(fn `AI_Check_Rotation`
  (params (min :type "Float (double-precision)") (max :type "Float (double-precision)") (angle :type "Float (double-precision)")))

(fn `AI_Control`
  (locals (cur_point :type "Vector Structure") (cur_distance :type "Float (double-precision)") (tmp_index :type Integer) (tmp_lf_flag :type Integer) (tmp_rf_flag :type Integer) (tmp_steer_flag :type Integer) (correction_needed :type Boolean))
  (bind _visited_spline_points (`self.Visited Spline Points`))
  (bind _returnvalue (`KismetMathLibrary.MakeVector` (`self.UE Lattitude`) (`self.UE Longtitude`)))
  (for (_ _array_index) _visited_spline_points
    (set `local.tmp_index` _array_index)
    (bind _returnvalue_2 (`KismetMathLibrary.MakeVector` (.x (`SplineComponent.GetLocationAtSplinePoint` (`/Game/BPs/2D/PathStuff/Path.Spline` (`self.Path`)) _array_index "Local")) (.y (`SplineComponent.GetLocationAtSplinePoint` (`/Game/BPs/2D/PathStuff/Path.Spline` (`self.Path`)) _array_index "Local"))))
    (bind _output_get (set `local.cur_distance` (`KismetMathLibrary.Vector_Distance` _returnvalue_2 _returnvalue)))
    (if (== (`|GetArrayItem` _visited_spline_points _array_index) 0)
      (bind _returnvalue_3 (`KismetMathLibrary.DegAcos` (`KismetMathLibrary.DotProduct2D` (`KismetMathLibrary.Normal2D` (`KismetMathLibrary.MakeVector2D` (.x (`SceneComponent.GetForwardVector` (`self.MainBox`))) (.y (`SceneComponent.GetForwardVector` (`self.MainBox`))))) (`KismetMathLibrary.Normal2D` (`KismetMathLibrary.MakeVector2D` (.x (- _returnvalue_2 _returnvalue)) (.y (- _returnvalue_2 _returnvalue)))))))
      (if (<= _returnvalue_3 87.0) :!label _label
        (bind _flag (`self.AI Increase Force` (`self.left_force`) 1.4 (`self.maxForce`) true))
        (bind _output_get_2 (set `local.tmp_lf_flag` _flag))
        (bind _flag_2 (`self.AI Increase Force` (`self.right_force`) 1.4 (`self.minForce`)))
        (bind _output_get_3 (set `local.tmp_rf_flag` _flag_2))
        (`self.AI_Forces` _output_get_2 _output_get_3 3)
        (set `local.correction_needed` true)
        (break)
        (elif (>= _returnvalue_3 93.0)
          (bind _flag_3 (`self.AI Increase Force` (`self.left_force`) 1.4 (`self.minForce`)))
          (bind _output_get_4 (set `local.tmp_lf_flag` _flag_3))
          (bind _flag_4 (`self.AI Increase Force` (`self.right_force`) 1.4 (`self.maxForce`) true))
          (bind _output_get_5 (set `local.tmp_rf_flag` _flag_4))
          (`self.AI_Forces` _output_get_4 _output_get_5 3)
          (set `local.correction_needed` true)
          (break)
          (else
            (`self.AI_Forces` 3 3 3)
            (`KismetArrayLibrary.Array_Set` (`self.Visited Spline Points`) (`local.tmp_index`) 1)
            (break))))
      (elif (== (`|GetArrayItem` _visited_spline_points _array_index) 1)
        (if (<= _output_get 5000.0)
          (`self.AI_Forces` 3 3 3)
          (`KismetArrayLibrary.Array_Set` _visited_spline_points (`local.tmp_index`) 2)
          (else
            (`|ExecutionSequence`
              (:`then_0`
                (set `local.correction_needed` false))
              (:`then_1`
                (goto _label))
              (:`then_2`
                (if (not (`local.correction_needed`))
                  (bind _flag_5 (`self.AI Increase Force` (`self.left_force`) 1.4 (`self.maxForce`) true))
                  (bind _output_get_6 (set `local.tmp_lf_flag` _flag_5))
                  (bind _flag_6 (`self.AI Increase Force` (`self.right_force`) 1.4 (`self.maxForce`) true))
                  (bind _output_get_7 (set `local.tmp_rf_flag` _flag_6))
                  (`self.AI_Forces` _output_get_6 _output_get_7 3)
                  (break))))))))))

(fn `AI_Forces`
  (params (Left_Force :type Integer) (Right_Force :type Integer) (Steer :type Integer))
  (bind _forcesflag (`self.ForcesFlag`))
  ;[1 1 1] 0: Release
  ; 1: Front
  ; 2: Back
  ; 3: Zero
  (`KismetArrayLibrary.Array_Set` _forcesflag 0 Left_Force)
  (`KismetArrayLibrary.Array_Set` _forcesflag 1 Right_Force)
  (set `self.SteeringFlag` Steer))

(fn `Apply Forces`
  (bind _returnvalue (* (* (`KismetMathLibrary.Normal` (`KismetMathLibrary.RotateAngleAxis` (`KismetMathLibrary.Conv_RotatorToVector` (`SceneComponent.K2_GetComponentRotation` (`self.ShipMainBody`))) 90.0 (0.0 0.0 1.0))) (`self.force_scaling`)) (`self.right_force`)))
  (bind _returnvalue_2 (* (* (`KismetMathLibrary.Normal` (`KismetMathLibrary.RotateAngleAxis` (`KismetMathLibrary.Conv_RotatorToVector` (`SceneComponent.K2_GetComponentRotation` (`self.ShipMainBody`))) 90.0 (0.0 0.0 1.0))) (`self.force_scaling`)) (`self.left_force`)))
  (`|ExecutionSequence`
    (:`then_0`
      (`PrimitiveComponent.AddForceAtLocation` (`self.MainBox`) _returnvalue_2 (`SceneComponent.K2_GetComponentLocation` (`self.Left Force Point`)) "None")
      (`SceneComponent.K2_SetWorldRotation` (`self.ArrowL`) (`KismetMathLibrary.Conv_VectorToRotator` _returnvalue_2) false false))
    (:`then_1`
      (`PrimitiveComponent.AddForceAtLocation` (`self.MainBox`) _returnvalue (`SceneComponent.K2_GetComponentLocation` (`self.Right Force Point`)) "None")
      (`SceneComponent.K2_SetWorldRotation` (`self.ArrowR`) (`KismetMathLibrary.Conv_VectorToRotator` _returnvalue) false false))
    (:`then_2`
      (`PrimitiveComponent.AddForceAtLocation` (`self.MainBox`) (* (* (`self.GetActorForwardVector`) (`self.force_scaling`)) (`self.steering force`)) (`SceneComponent.K2_GetComponentLocation` (`self.Steering Point`)) "None"))))

(fn `Calculate_Path`
  (locals (temp_var :type Integer) (tmp_dist :type "Float (double-precision)")))

(fn `Initialize_Ship`)

(fn `Radar`)

(fn `SetForces`
  (bind _steeringflag (`self.SteeringFlag`))
  (bind _left_force (`self.left_force`))
  (bind _right_force (`self.right_force`))
  (bind _steering_perc (`self.steering perc`))
  (bind _forcesflag (`self.ForcesFlag`))
  (bind _forcesflag_2 (`self.ForcesFlag`))
  (bind _steering_perc_2 (`self.steering perc`))
  (bind _output (`|GetArrayItem` _forcesflag 1))
  (bind _output_2 (`|GetArrayItem` _forcesflag_2))
  (`|ExecutionSequence`
    (:`then_0`
      (if (> _output_2 0)
        (if (== _output_2 3)
          (if (== _left_force 0.0)
            (`KismetArrayLibrary.Array_Set` _forcesflag_2)
            (elif (< _left_force 0.0)
              (set `self.left_force` (`KismetMathLibrary.FMin` (+ _left_force (`self.decel_step`))))
              (else
                (set `self.left_force` (`KismetMathLibrary.FMax` (- _left_force (`self.decel_step`)))))))
          (elif (== _output_2 1)
            (set `self.left_force` (`KismetMathLibrary.FMin` (+ (`self.left_force`) (`self.accel_step`)) (`self.maxForce`)))
            (else
              (set `self.left_force` (`KismetMathLibrary.FMax` (- (`self.left_force`) (`self.accel_step`)) (`self.minForce`))))))))
    (:`then_1`
      (if (> _output 0)
        (if (== _output 3)
          (if (== _right_force 0.0)
            (`KismetArrayLibrary.Array_Set` _forcesflag 1)
            (elif (< _right_force 0.0)
              (set `self.right_force` (`KismetMathLibrary.FMin` (+ _right_force (`self.decel_step`))))
              (else
                (set `self.right_force` (`KismetMathLibrary.FMax` (- _right_force (`self.decel_step`)))))))
          (elif (== _output 1)
            (set `self.right_force` (`KismetMathLibrary.FMin` (+ (`self.right_force`) (`self.accel_step`)) (`self.maxForce`)))
            (else
              (set `self.right_force` (`KismetMathLibrary.FMax` (- (`self.right_force`) (`self.accel_step`)) (`self.minForce`))))))))
    (:`then_2`
      (`|ExecutionSequence`
        (:`then_0`
          (if (> _steeringflag 0)
            (if (== _steeringflag 3)
              (if (== _steering_perc_2 0.0)
                (set `self.SteeringFlag` 0)
                (elif (< _steering_perc_2 0.0)
                  (set `self.steering perc` (`KismetMathLibrary.FMin` (+ (`self.steering perc`) (`self.dec_steering_step`))))
                  (else
                    (set `self.steering perc` (`KismetMathLibrary.FMax` (- (`self.steering perc`) (`self.dec_steering_step`)))))))
              (elif (== _steeringflag 1)
                (set `self.steering perc` (`KismetMathLibrary.FMax` (- (`self.steering perc`) (`self.inc_steering_step`)) (`self.minSteeringPerc`)))
                (else
                  (set `self.steering perc` (`KismetMathLibrary.FMin` (+ (`self.steering perc`) (`self.inc_steering_step`)) (`self.maxSteeringPerc`))))))))
        (:`then_1`
          (if (!= _steering_perc 0.0)
            (if (< _steering_perc 0.0)
              (set `self.steering force` (+ (* (* (`self.left_force`) (`self.steering perc`)) 2.0) (* (`self.right_force`) (`self.steering perc`))))
              (else
                (set `self.steering force` (+ (* (`self.left_force`) (`self.steering perc`)) (* (* (`self.right_force`) (`self.steering perc`)) 2.0)))))))))))

(fn `Toggle Cameras`
  (params (new_cam :type Integer))
  (bind _camera_free (`self.Camera FREE`))
  (bind _camera_c (`self.Camera C`))
  (bind _camera_r (`self.Camera R`))
  (bind _camera_nw (`self.Camera NW`))
  (bind _camera_n (`self.Camera N`))
  (bind _camera_ne (`self.Camera NE`))
  (bind _camera_s (`self.Camera S`))
  (bind _camera_se (`self.Camera SE`))
  (bind _camera_sw (`self.Camera SW`))
  (bind _camera_l (`self.Camera L`))
  (if (`self.IsPlayerControlled`)
    (for _array_element (`self.GetComponentsByTag` "/Script/Engine.CameraComponent" (`|GetArrayItem` (`self.Name_Tag`)))
      (`ActorComponent.SetActive` _array_element false false)
      (set `ActorComponent.ComponentTags` (`self.Empty_Tag`) _array_element))
    (switch `int` new_cam
      (:`Default`
        (`ActorComponent.SetActive` (`self.Camera FREE`) true false))
      (:`0`
        (`ActorComponent.SetActive` _camera_free true false)
        (set `ActorComponent.ComponentTags` (`self.Name_Tag`) _camera_free))
      (:`1`
        (`ActorComponent.SetActive` _camera_sw true false)
        (set `ActorComponent.ComponentTags` (`self.Name_Tag`) _camera_sw))
      (:`2`
        (`ActorComponent.SetActive` _camera_s true false)
        (set `ActorComponent.ComponentTags` (`self.Name_Tag`) _camera_s))
      (:`3`
        (`ActorComponent.SetActive` _camera_se true false)
        (set `ActorComponent.ComponentTags` (`self.Name_Tag`) _camera_se))
      (:`4`
        (`ActorComponent.SetActive` _camera_l true false)
        (set `ActorComponent.ComponentTags` (`self.Name_Tag`) _camera_l))
      (:`5`
        (`ActorComponent.SetActive` _camera_c true false)
        (set `ActorComponent.ComponentTags` (`self.Name_Tag`) _camera_c))
      (:`6`
        (`ActorComponent.SetActive` _camera_r true false)
        (set `ActorComponent.ComponentTags` (`self.Name_Tag`) _camera_r))
      (:`7`
        (`ActorComponent.SetActive` _camera_nw true false)
        (set `ActorComponent.ComponentTags` (`self.Name_Tag`) _camera_nw))
      (:`8`
        (`ActorComponent.SetActive` _camera_n true false)
        (set `ActorComponent.ComponentTags` (`self.Name_Tag`) _camera_n))
      (:`9`
        (`ActorComponent.SetActive` _camera_ne true false)
        (set `ActorComponent.ComponentTags` (`self.Name_Tag`) _camera_ne)))))

(fn `updateLonLat`)

(fn `UserConstructionScript`)

(fn `ZoomInOut`
  (params (isout :type Boolean))
  (locals (`Max FoV` :type "Float (double-precision)" :default 150.0) (`FoV Step` :type "Float (double-precision)") (`Min FoV` :type "Float (double-precision)" :default 10.0))
  (bind _returnvalue (`self.GetComponentsByTag` "/Script/Engine.CameraComponent" (`|GetArrayItem` (`self.Name_Tag`))))
  (bind _output (`|GetArrayItem` _returnvalue))
  (bind _returnvalue_2 (+ (`CameraComponent.FieldOfView` _output) (`local.FoV Step`)))
  (if (`self.IsPlayerControlled`)
    (if (> (`KismetArrayLibrary.Array_Length` _returnvalue) 0)
      (if isout
        (set `local.FoV Step` 3.0)
        (set `CameraComponent.FieldOfView` (`KismetMathLibrary.FMin` _returnvalue_2 (`local.Max FoV`)) _output)
        (else
          (set `local.FoV Step` -3.0)
          (set `CameraComponent.FieldOfView` (`KismetMathLibrary.FMax` _returnvalue_2 (`local.Min FoV`)) _output))))))