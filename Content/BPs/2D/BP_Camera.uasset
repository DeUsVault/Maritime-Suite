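; BP_Camera is an orthographic camera Blueprint for a 2D map view, with helpers for bounds and geographic coordinates.
; GetCoordinates deprojects the mouse to world space, linearly remaps it to latitude and longitude from hard-coded calibration points, and prints the result.
; ClampCamera limits only the X position to fixed edges inset by half the OrthoWidth.
; The event graph is empty, so neither function is called within this Blueprint.
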(event `self.ReceiveTick`
  (params (DeltaSeconds :type "Float (single-precision)")))

(fn `Clamp_Camera`
  (bind _camera (`self.Camera`))
  (bind (_returnvalue_x _returnvalue_y _returnvalue_z) (`KismetMathLibrary.BreakVector` (`SceneComponent.K2_GetComponentLocation` _camera)))
  (`SceneComponent.K2_SetWorldLocation` (`self.Camera`) (`KismetMathLibrary.MakeVector` (`KismetMathLibrary.FClamp` _returnvalue_x (+ 187514.0 (/ (`CameraComponent.OrthoWidth` _camera) 2.0)) (- 1551114.0 (/ (`CameraComponent.OrthoWidth` _camera) 2.0))) _returnvalue_y _returnvalue_z) false false))

(fn `Get_Coordinates`
  (bind _worldlocation (`PlayerController.DeprojectMousePositionToWorld` (`GameplayStatics.GetPlayerController` 0)))
  (`KismetSystemLibrary.PrintString` (`KismetStringLibrary.Concat_StrStr` "Lat : " (`KismetStringLibrary.Conv_DoubleToString` (`KismetMathLibrary.Lerp` 41.121 33.0 (/ (- (.y _worldlocation) 11547.429) (- 866483.447 11547.429)))) " Long : " (`KismetStringLibrary.Conv_DoubleToString` (`KismetMathLibrary.Lerp` 18.515 34.759 (/ (- (.x _worldlocation) 207567.615) (- 1530015.13 207567.615))))) true true (struct :`G` 0.354062 :`B` 0.536458 :`A` 1.0) 1.0))

(fn `UserConstructionScript`)