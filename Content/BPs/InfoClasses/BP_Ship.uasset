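; BP_Ship is an info class for a ship that holds its radar object and feeds the ship's details widget.
; UpdateRadarObject clears the radar when the incoming name is empty, otherwise updates the existing BP_Radar or constructs one, using the name as a provisional validity check.
; Initialise stores the details widget, and UpdateWidgetInfo runs the parent update, then passes Info to WBP_ShipAssetDetails.
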(fn `Initialise`
  (params (DetailsWidget :type "/Game/Blueprints/HUDStuff/AssetDetailsWidgets/WBP_ShipAssetDetails Object Reference"))
  (set `self.DetailsWidget` DetailsWidget)
  (`self.UpdateWidgetInfo`))

(fn `UpdateRadarObject`
  (params (RadarInfo :type "/Game/Assets/Data/F_RadarComponent Structure (by ref)"))
  (bind _radar (`self.Radar`))
  (if (== (`KismetStringLibrary.Len` (`KismetTextLibrary.Conv_TextToString` (`.Name_10_55EE3B8D42F38D8C4AB2F4BD744DA81B` (break `/Game/Assets/Data/F_ComponentGeneralDetails` (`.GeneralDetails_2_4ED183B74E1793CBD18D579D67B5B4F8` (break `/Game/Assets/Data/F_RadarComponent` RadarInfo)))))) 0)
    (set `self.Radar` null)
    (elif (`KismetSystemLibrary.IsValid` _radar)
      (set `/Game/BPs/InfoClasses/BP_Radar.RadarInfo` RadarInfo _radar)
      (else
        (bind _returnvalue (`|GenericCreateObject` "/Game/BPs/InfoClasses/BP_Radar.BP_Radar_C" RadarInfo))
        (set `self.Radar` _returnvalue)))))

(fn `UpdateWidgetInfo`
  (`parent.UpdateWidgetInfo`)
  (bind _aswbp_ship_asset_details (cast `/Game/Blueprints/HUDStuff/AssetDetailsWidgets/WBP_ShipAssetDetails` (`self.DetailsWidget`)))
  (`/Game/Blueprints/HUDStuff/AssetDetailsWidgets/WBP_ShipAssetDetails.SetShipDetails` _aswbp_ship_asset_details (`self.Info`)))