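; HUD for the asset customization level that creates the customization screen widget and links it to the rotating platform and the displayed ship.
; On BeginPlay it finds the platform and the "vehicle"-tagged BP_ShipActor, then binds the widget's dispatchers.
; Rotation presses start and stop the platform, and vehicle selection rebuilds the ship from the chosen object.
; Component clicks update the ship's radar from general details only, flagged as needing a fix, while sonar just prints.
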(event `self.ReceiveBeginPlay`
  (bind _outactors (`GameplayStatics.GetAllActorsOfClass` "/Game/Blueprints/AssetCustomizationLevel/BP_RotatingPlatform_Blueprint.BP_RotatingPlatform_Blueprint_C"))
  (set `self.RotatingPlatform` (`|GetArrayItem` _outactors))
  (bind _outactors_2 (`GameplayStatics.GetAllActorsWithTag` "vehicle"))
  (bind _asbp_ship_actor (cast `/Game/Assets/Data/BP_ShipActor` (`|GetArrayItem` _outactors_2)))
  (set `self.Vehicle` _asbp_ship_actor)
  (bind _returnvalue (`|CreateWidget` "/Game/Blueprints/HUDStuff/AssetCustomisationScreen/WBP_CustomizationScreenHUD.WBP_CustomizationScreenHUD_C" (`GameplayStatics.GetPlayerController` 0)))
  (add `/Game/Blueprints/HUDStuff/AssetCustomisationScreen/WBP_VehicleList.OnVehicleSelected` (`/Game/Blueprints/HUDStuff/AssetCustomisationScreen/WBP_CustomizationScreenHUD.VehicleList` _returnvalue) (delegate `OnVehicleSelected_Event`))
  (add `/Game/Blueprints/HUDStuff/AssetCustomisationScreen/WBP_CustomizationScreenHUD.RotationPressedDispatcher` _returnvalue (delegate `RotationPressedDispatcher_Event_0`))
  (add `/Game/Blueprints/HUDStuff/AssetCustomisationScreen/WBP_CustomizationScreenHUD.RotationReleasedDispatcher` _returnvalue (delegate `RotationReleasedDispatcher_Event_0`))
  (add `/Game/Blueprints/HUDStuff/AssetCustomisationScreen/WBP_ComponentSelection.ComponentClickedDispatcher` (`/Game/Blueprints/HUDStuff/AssetCustomisationScreen/WBP_CustomizationScreenHUD.WBP_ComponentSelection` _returnvalue) (delegate `ComponentClickedDispatcher_Event_0`))
  (`UserWidget.AddToViewport` _returnvalue 0))

(event `RotationPressedDispatcher_Event_0`
  (params (IsRotatingLeft :type Boolean))
  (`/Game/Blueprints/AssetCustomizationLevel/BP_RotatingPlatform_Blueprint.RotationStart` (`self.RotatingPlatform`) IsRotatingLeft))

(event `RotationReleasedDispatcher_Event_0`
  (`/Game/Blueprints/AssetCustomizationLevel/BP_RotatingPlatform_Blueprint.RotationEnd` (`self.RotatingPlatform`)))

(event `ComponentClickedDispatcher_Event_0`
  (params (Details :type "/Game/Assets/Data/F_ComponentGeneralDetails Structure") (ComponentType :type "/Game/Assets/Data/ShipComponentType Enum" :default "NewEnumerator0"))
  (switch `/Game/Assets/Data/ShipComponentType` ComponentType
    (:`NewEnumerator0`
      (`/Game/Assets/Data/BP_ShipActor.UpdateRadarComponent` (`self.Vehicle`) (make `/Game/Assets/Data/F_RadarComponent` :`GeneralDetails` Details :`Class` null)))
    (:`NewEnumerator1`
      (`KismetSystemLibrary.PrintString` (`KismetStringLibrary.Concat_StrStr` "UPDATE SONAR with " (`KismetTextLibrary.Conv_TextToString` (`.Name_10_55EE3B8D42F38D8C4AB2F4BD744DA81B` (break `/Game/Assets/Data/F_ComponentGeneralDetails` Details))))))))

(event `OnVehicleSelected_Event`
  (params (ShipObject :type "/Game/BPs/InfoClasses/BP_Ship Object Reference"))
  (`/Game/Assets/Data/BP_ShipActor.UpdateActorFromObject` (`self.Vehicle`) ShipObject))

(fn `UserConstructionScript`)