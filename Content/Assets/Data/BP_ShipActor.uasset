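; BP_ShipActor is the actor representation of a ship data object, showing its hull mesh and radar.
; UpdateActorFromObject applies the mesh from the ship's info, spawns the radar through a child actor component attached at the mesh's RadarSocket, and stores the object.
; Missing data clears the mesh or radar.
; UpdateRadarComponent writes new radar info to the ship object, then refreshes the actor from it.
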(fn `AttachRadarComponent`)

(fn `GetMesh`)

(fn `UpdateActorFromObject`
  (params (ShipObject :type "/Game/BPs/InfoClasses/BP_Ship Object Reference"))
  (bind _radar (`self.Radar`))
  (bind _generaldetails (break `/Game/Assets/Data/F_Ships` (`/Game/BPs/InfoClasses/BP_Ship.Info` ShipObject)))
  (bind _childactor (`ChildActorComponent.ChildActor` _radar))
  (if (`KismetSystemLibrary.IsValid` ShipObject)
    (if (`KismetSystemLibrary.IsValid` (`.Mesh_21_BE1551E449CD2166133CA19D0094EC94` (break `/Game/Assets/Data/F_ComponentGeneralDetails` _generaldetails)))
      (`StaticMeshComponent.SetStaticMesh` (`self.StaticMesh`) (`.Mesh_21_BE1551E449CD2166133CA19D0094EC94` (break `/Game/Assets/Data/F_ComponentGeneralDetails` _generaldetails)))
      (if (`KismetSystemLibrary.IsValid` (`/Game/BPs/InfoClasses/BP_Ship.Radar` ShipObject))
        (`ChildActorComponent.SetChildActorClass` _radar "/Game/BPs/2D/Radar/rotator/Radar.Radar_C")
        (cast `/Game/BPs/2D/Radar/rotator/Radar` _childactor)
        (`self.K2_AttachToComponent` _childactor (`self.StaticMesh`) "RadarSocket" "KeepRelative" "KeepRelative" "KeepRelative" true)
        (else
          (`ChildActorComponent.SetChildActorClass` _radar null :!label _label)))
      (else
        (`StaticMeshComponent.SetStaticMesh` (`self.StaticMesh`) null :!label _label_2)
        (goto _label)))
    (else
      (goto _label_2)))
  (set `self.ShipObject` ShipObject))

(fn `UpdateRadarComponent`
  (params (RadarInfo :type "/Game/Assets/Data/F_RadarComponent Structure"))
  (bind _shipobject (`self.ShipObject`))
  (`/Game/BPs/InfoClasses/BP_Ship.UpdateRadarObject` _shipobject RadarInfo)
  (`self.UpdateActorFromObject` _shipobject))

(fn `UserConstructionScript`)